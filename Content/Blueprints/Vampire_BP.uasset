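; Vampire enemy Blueprint that shows its Health on a widget-based health bar.
; On actor overlap, it casts the EnemyHealth component's widget to Enemy_UI_BP and caches the reference.
; Each Tick, once that reference is valid, it sets the bar's percent from Health on a 100-point scale, so updates begin only after a first overlap.
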(event `self.ReceiveActorBeginOverlap`
  (params (OtherActor :type "Actor Object Reference"))
  (bind _asenemy_ui_bp (cast `/Game/Blueprints/Enemy_UI_BP` (`WidgetComponent.GetUserWidgetObject` (`self.EnemyHealth`))))
  (set `self.Enemy UI BP REF` _asenemy_ui_bp))

(event `self.ReceiveTick`
  (params (DeltaSeconds :type "Float (single-precision)"))
  (bind _enemy_ui_bp_ref (`self.Enemy UI BP REF`))
  (`/Engine/EditorBlueprintResources/StandardMacros.IsValid` _enemy_ui_bp_ref
    (:`Is Valid`
      (`ProgressBar.SetPercent` (`/Game/Blueprints/Enemy_UI_BP.Enemyhealthbar` _enemy_ui_bp_ref) (/ (`self.Health`) 100.0)))))

(fn `UserConstructionScript`)